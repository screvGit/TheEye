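; Interactable teleporter actor that sends the player to a target level.
; On BeginPlay, a Hover timeline bobs and spins the Crystal component.
; Interacting stores the teleporter's TeleTag in the main game instance so it carries across the level change, then opens TargetLevel.
; LookAt only prints a "Travel" prompt through PrintString and returns an empty string.
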(event EventInteractwith
  (params (PlayerCharacter :type BP%20First%20Person%20Character%20Object%20Reference))
  (bind _asmain_game_instane_bp (Utilities|Casting|CastToMainGameInstane_Bp (Game|GetGameInstance)))
  (Variables|/Game/MainGameInstane_Bp.MainGameInstane_Bp_C|SetTeleportationTag _asmain_game_instane_bp (Variables|Default|GetTeleTag))
  (Game|OpenLevel(byObjectReference) (Variables|Default|GetTargetLevel)))

(event EventBeginPlay
  (bind _crystal (Variables|Default|GetCrystal))
  (bind _crystal_2 (Variables|Default|GetCrystal))
  (bind _returnvalue (Transformation|GetRelativeTransform _crystal))
  (bind _returnvalue_2 (Transformation|GetRelativeTransform _crystal_2))
  (bind (_direction _hovertrack _spintrack) (Timeline|Hover Play)
    (:Update
      (Transformation|SetRelativeLocation _crystal (Math|Vector|MakeVector (.x (.location _returnvalue)) (.y (.location _returnvalue)) (Math|Float|Lerp 0.0 1e+01 _hovertrack)) false false)
      (Transformation|SetRelativeRotation _crystal_2 (Math|Rotator|MakeRotator (.roll (.rotation _returnvalue_2)) (.pitch (.rotation _returnvalue_2)) (Math|Float|Lerp 0.0 3.6e+02 _spintrack)) false false))))

(fn ConstructionScript)

(fn Lookat
  (Development|PrintString "Travel")
  (return ""))