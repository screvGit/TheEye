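; Double door actor that swings two door meshes open when interacted with and returns "Door" as its look-at text.
; One timeline drives shortest-path rotation lerps between each door's closed and open rotations, toggling IsOpen when finished.
; Interactwith only opens a closed door, at a play rate set from TimeToOpenS.
; CloseDoor reverses the timeline, but its only caller here, with the TimeToCloseS rate, is disconnected.
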(event Custom|Open%20Door
  (bind _door_track (Timeline|Open%20Door%20T Play)
    (:Update
      (Transformation|SetRelativeRotation (Variables|Default|GetDoor1) (Math|Rotator|Lerp(Rotator) (Variables|Default|GetD1ClosePosition) (Variables|Default|GetD1OpenPosition) _door_track true) false false)
      (Transformation|SetRelativeRotation (Variables|Default|GetDoor%202) (Math|Rotator|Lerp(Rotator) (Variables|Default|GetD2ClosePosition) (Variables|Default|GetD2OpenPosition) _door_track true) false false))
    (:Finished
      (Variables|Default|SetIsOpen (not (Variables|Default|GetIsOpen))))))

(event Custom|Close%20Door
  (bind _door_track (Timeline|Open%20Door%20T Reverse)
    (:Update
      (Transformation|SetRelativeRotation (Variables|Default|GetDoor1) (Math|Rotator|Lerp(Rotator) (Variables|Default|GetD1ClosePosition) (Variables|Default|GetD1OpenPosition) _door_track true) false false)
      (Transformation|SetRelativeRotation (Variables|Default|GetDoor%202) (Math|Rotator|Lerp(Rotator) (Variables|Default|GetD2ClosePosition) (Variables|Default|GetD2OpenPosition) _door_track true) false false))
    (:Finished
      (Variables|Default|SetIsOpen (not (Variables|Default|GetIsOpen))))))

(event EventInteractwith
  (params (PlayerCharacter :type BP%20First%20Person%20Character%20Object%20Reference))
  (if (not (Variables|Default|GetIsOpen))
    (Components|Timeline|SetPlayRate (Variables|Default|GetOpen%20Door%20T) (Variables|Default|GetTimeToOpen%28s%29))
    (CallFunction|OpenDoor)))

(fn ConstructionScript)

(fn Lookat
  (return "Door"))