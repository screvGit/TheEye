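; Food pickup, a cooked chicken mesh that the first-person character can eat through Interact.
; A collision overlap caches the BP_FirstPersonCharacter reference, which Eat uses instead of the Interactor passed in.
; Eat checks the Eaten flag, passes FoodValue to the character's EatFood and hides the chicken mesh.
; The graphs never set Eaten, and the actor is hidden rather than destroyed.
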(event OnComponentBeginOverlap(Collision)
  (params (OverlappedComponent :type Primitive%20Component%20Object%20Reference) (OtherActor :type Actor%20Object%20Reference) (OtherComp :type Primitive%20Component%20Object%20Reference) (OtherBodyIndex :type Integer) (bFromSweep :type Boolean) (SweepResult :type Hit%20Result%20Structure%20%28by%20ref%29))
  (bind _asbp_first_person_character (Utilities|Casting|CastToBP_FirstPersonCharacter OtherActor))
  (Variables|Default|SetCharRef _asbp_first_person_character))

(event Custom|Eat
  (if (not (Variables|Default|GetEaten))
    (Default|EatFood (Variables|Default|GetCharRef) (Variables|Default|GetFoodValue))
    (Rendering|SetVisibility (Variables|Default|GetCookedChicken) false false)))

(fn ConstructionScript)

(fn Interact
  (params (Interactor :type Character%20Object%20Reference))
  (CallFunction|Eat)
  (return false))